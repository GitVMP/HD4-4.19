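; Screen actor that shows a localized image between levels for seven seconds, then destroys itself.
; On BeginPlay it reads the IsFrench flag from HD4_GI and picks the French or English material map.
; It looks up the current level name in that map and applies the material to ScreenBetweenLevels; a failed game instance cast skips everything, including the destroy.
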(event `self.ReceiveBeginPlay`
  (bind _ashd4_gi (cast `/Game/HD4_GI` (`GameplayStatics.GetGameInstance`)))
  (if (`/Game/HD4_GI.Is French?` _ashd4_gi)
    (bind _returnvalue (`GameplayStatics.GetCurrentLevelName` true))
    (`PrimitiveComponent.SetMaterial` (`self.Screen-Between-Levels`) 0 (`BlueprintMapLibrary.Map_Find` (`self.French Mats`) _returnvalue))
    (else
      (bind _returnvalue_2 (`GameplayStatics.GetCurrentLevelName` true))
      (`PrimitiveComponent.SetMaterial` (`self.Screen-Between-Levels`) 0 (`BlueprintMapLibrary.Map_Find` (`self.English Mats`) _returnvalue_2))))
  (`KismetSystemLibrary.Delay` 7.0)
  (`self.K2_DestroyActor`))

(fn `UserConstructionScript`)