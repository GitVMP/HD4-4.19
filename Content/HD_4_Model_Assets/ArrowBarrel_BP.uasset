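; ArrowBarrel_BP is a barrel-with-arrows actor that counts as a hit on the player's boat when touched.
; On BeginPlay a timeline drives the Z offset of the BarrelArrowsDM mesh to move it vertically.
; When a PawnBoat2 overlaps the capsule, a hit sound plays and, through a DoOnce, the boat's HitNum increments before the actor destroys itself after a one-second delay.
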(event `self.ReceiveBeginPlay`
  (bind (_direction _newtrack_1) (`Timeline|Timeline_0`)
    (:`Update`
      (`SceneComponent.K2_SetRelativeLocationAndRotation` (`self.BarrelArrows_DM`) (`KismetMathLibrary.MakeVector` 0.0 0.0 _newtrack_1) (`KismetMathLibrary.MakeRotator` 0.0) false false))))

(event `self.Capsule.OnComponentBeginOverlap`
  (params (OverlappedComponent :type "PrimitiveComponent Object Reference") (OtherActor :type "Actor Object Reference") (OtherComp :type "PrimitiveComponent Object Reference") (OtherBodyIndex :type Integer) (bFromSweep :type Boolean) (SweepResult :type "HitResult Structure (by ref)"))
  (bind _aspawn_boat_2 (cast `/Game/PawnBoat2` OtherActor))
  (`GameplayStatics.PlaySound2D` "/Game/HD_4_Model_Assets/HD-4-Sounds/Hit_Barrel_01-Mono.Hit_Barrel_01-Mono")
  (`/Engine/EditorBlueprintResources/StandardMacros.DoOnce` false
    (:`Completed`
      (bind _result (`/Engine/EditorBlueprintResources/StandardMacros.IncrementInt` (`/Game/PawnBoat2.Hit Num` _aspawn_boat_2))
        (:`  `
          (set `/Game/PawnBoat2.Hit Num` _result _aspawn_boat_2)
          (`KismetSystemLibrary.Delay` 1.0)
          (`self.K2_DestroyActor`))))))

(fn `UserConstructionScript`)